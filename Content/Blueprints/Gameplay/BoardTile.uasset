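; BoardTile is a hexagonal board tile actor that configures its look in the construction script.
; IsHighGround selects the high or standard hex mesh, then SetMaterialByArena applies a material to the first slot.
; That function switches on CurrentArenaMap, resetting Empty to the debug arena, but every arena currently uses the same rock material for high ground and muddy grass otherwise.
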(event EventBeginPlay)

(event Collision|EventActorBeginOverlap
  (params (OtherActor :type Actor%20Object%20Reference)))

(event EventTick
  (params (DeltaSeconds :type Float%20%28single-precision%29)))

(fn ConstructionScript
  (bind _tilemesh (Variables|Default|GetTileMesh))
  (if (Variables|Default|GetbIsHighGround)
    (bind _returnvalue (Components|StaticMesh|SetStaticMesh _tilemesh "/Game/Meshes/Board/HexagonTile_High.HexagonTile_High"))
    (else
      (bind _returnvalue_2 (Components|StaticMesh|SetStaticMesh _tilemesh "/Game/Meshes/Board/HexagonTile.HexagonTile"))))
  (if (or _returnvalue _returnvalue_2)
    (CallFunction|SetMaterialbyArena)))

(fn SetMaterialbyArena
  (bind _tilemesh (Variables|Default|GetTileMesh))
  (bind _bishighground (Variables|Default|GetbIsHighGround))
  (switch Utilities|FlowControl|Switch|SwitchonEArenaList (Variables|Default|GetCurrentArenaMap)
    (:Arena_Empty
      (Variables|Default|SetCurrentArenaMap "Arena_Debug")
      (Rendering|Material|SetMaterial _tilemesh 0 (select (Variables|Default|GetbIsHighGround) "/Game/Materials/Board/M_Rock_CrumblingCliffShrubs_Inst.M_Rock_CrumblingCliffShrubs_Inst" "/Game/Materials/Board/M_Grass_Muddy_Inst.M_Grass_Muddy_Inst") :!label _label))
    (:Arena_Debug
      (goto _label))
    (:Arena_UrbanTheater
      (Rendering|Material|SetMaterial _tilemesh 0 (select _bishighground "/Game/Materials/Board/M_Rock_CrumblingCliffShrubs_Inst.M_Rock_CrumblingCliffShrubs_Inst" "/Game/Materials/Board/M_Grass_Muddy_Inst.M_Grass_Muddy_Inst")))
    (:Arena_MountainRange
      (Rendering|Material|SetMaterial _tilemesh 0 (select _bishighground "/Game/Materials/Board/M_Rock_CrumblingCliffShrubs_Inst.M_Rock_CrumblingCliffShrubs_Inst" "/Game/Materials/Board/M_Grass_Muddy_Inst.M_Grass_Muddy_Inst")))
    (:Arena_Woodlands
      (Rendering|Material|SetMaterial _tilemesh 0 (select _bishighground "/Game/Materials/Board/M_Rock_CrumblingCliffShrubs_Inst.M_Rock_CrumblingCliffShrubs_Inst" "/Game/Materials/Board/M_Grass_Muddy_Inst.M_Grass_Muddy_Inst"))))
  (return))